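; Enemy character that hunts the player and triggers a jump scare on contact.
; A looping timer started on BeginPlay re-evaluates movement, chasing the player when a complete navmesh path exists, otherwise trying a random reachable point nearby.
; When IsMoving is false, each timer tick halts movement instead.
; Overlapping the first-person character briefly shows a scary-face widget with a laugh sound, without applying damage.
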(event `self.ReceiveBeginPlay`
  ;[1 1 1] Archie: Movement
  (`KismetSystemLibrary.K2_SetTimerDelegate` (delegate `Move`) 3.0 true))

(event `Move`
  (bind (_randomlocation _returnvalue) (`NavigationSystemV1.K2_GetRandomReachablePointInRadius` (`self.K2_GetActorLocation`) 2000.0 null null))
  ;[1 1 1] Archie: Movement
  (if (`self.isMoving`)
    (bind _returnvalue_2 (`NavigationSystemV1.FindPathToLocationSynchronously` (`NavigationSystemV1.K2_ProjectPointToNavigation` (`self.K2_GetActorLocation`) null null (`self.QueryExtent`)) (`NavigationSystemV1.K2_ProjectPointToNavigation` (`self.K2_GetActorLocation` (`GameplayStatics.GetPlayerPawn` 0)) null null (`self.QueryExtent`)) null null))
    (if (and (not (`NavigationPath.IsPartial` _returnvalue_2)) (`NavigationPath.IsValid` _returnvalue_2))
      (`|AIMoveTo` self (0.0 0.0 0.0) (`GameplayStatics.GetPlayerPawn` 0) 200.0)
      (elif _returnvalue
        (`|AIMoveTo` self (`NavigationSystemV1.K2_ProjectPointToNavigation` _randomlocation null null (`self.QueryExtent`)) null)))
    (else
      (`MovementComponent.StopMovementImmediately` (`self.CharacterMovement`)))))

(event `self.ReceiveActorBeginOverlap`
  (params (OtherActor :type "Actor Object Reference"))
  ;[1 1 1] Archie: Player Hit.... DO NOT KNOW WHAT TO DO WITH THIS
  (cast `/Game/FirstPersonBP/Blueprints/FirstPersonCharacter` OtherActor)
  (bind _returnvalue (`|CreateWidget` "/Game/UI/ScaryFaceJumpScare.ScaryFaceJumpScare_C"))
  (`UserWidget.AddToViewport` _returnvalue 0)
  (`GameplayStatics.PlaySound2D` "/Game/Audio/Laugh_1.Laugh_1" 1.0 1.0 0.0 null null)
  (`KismetSystemLibrary.Delay` 1.0)
  (`Widget.RemoveFromParent` _returnvalue))

(fn `UserConstructionScript`)