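; Battery pickup actor that spins continuously and recharges the first-person character's Battery when overlapped.
; On overlap with FirstPersonCharacter it adds 5 to Battery, tops values in the high nineties up to exactly 100, or adds nothing when already full.
; The pickup destroys itself in every case, even at full charge.
; Tick applies a fixed, frame-rate-dependent local rotation each frame.
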(event `self.ReceiveActorBeginOverlap`
  (params (OtherActor :type "Actor Object Reference"))
  (bind _asfirst_person_character (cast `/Game/FirstPersonBP/Blueprints/FirstPersonCharacter` OtherActor))
  (bind _battery (`/Game/FirstPersonBP/Blueprints/FirstPersonCharacter.battery` _asfirst_person_character))
  (if (and (>= _battery 95) (<= _battery 99))
    (set `/Game/FirstPersonBP/Blueprints/FirstPersonCharacter.battery` (+ _battery (- 100 _battery)) _asfirst_person_character)
    (`self.K2_DestroyActor`)
    (elif (== _battery 100)
      (set `/Game/FirstPersonBP/Blueprints/FirstPersonCharacter.battery` (+ _battery 0) _asfirst_person_character)
      (`self.K2_DestroyActor`)
      (else
        (set `/Game/FirstPersonBP/Blueprints/FirstPersonCharacter.battery` (+ _battery 5) _asfirst_person_character)
        (`self.K2_DestroyActor`)))))

(event `self.ReceiveTick`
  (params (DeltaSeconds :type "Float (single-precision)"))
  (`self.K2_AddActorLocalRotation` (struct :`Yaw` 1.0)))

(fn `UserConstructionScript`)