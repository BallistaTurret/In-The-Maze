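; Level 2 trigger volume that sets off a one-time enemy scare when the first-person player walks into it.
; On overlap it toggles IsMoving on an EnemyCharacter_BP assigned in the editor.
; The first overlap also plays a laugh, hides the player's flashlight for a few seconds, restores it, then destroys the trigger.
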(event `self.ReceiveTick`
  (params (DeltaSeconds :type "Float (single-precision)"))
  ;[1 1 1] Debugging
)

(event `self.ReceiveActorBeginOverlap`
  (params (OtherActor :type "Actor Object Reference"))
  ;[1 1 1] Once the Box is collides with, allow the movement to start
  (bind _asfirst_person_character (cast `/Game/FirstPersonBP/Blueprints/FirstPersonCharacter` OtherActor))
  (bind _asenemy_character_bp (cast `/Game/Blueprints/EnemyCharacter_BP` (`self.EnemyCharacterReference`)))
  (set `/Game/Blueprints/EnemyCharacter_BP.isMoving` (not (`/Game/Blueprints/EnemyCharacter_BP.isMoving` _asenemy_character_bp)) _asenemy_character_bp)
  (if (not (`self.hasWalked`))
    (`GameplayStatics.PlaySound2D` "/Game/Audio/Laugh_1.Laugh_1" 1.0 1.0 0.0 null null)
    (set `self.hasWalked` true)
    (bind _flashlight (`/Game/FirstPersonBP/Blueprints/FirstPersonCharacter.Flashlight` _asfirst_person_character))
    (`SceneComponent.SetVisibility` _flashlight false false)
    (`KismetSystemLibrary.Delay` 3.0)
    (`SceneComponent.SetVisibility` _flashlight true false)
    (`self.K2_DestroyActor`)))

(fn `UserConstructionScript`)