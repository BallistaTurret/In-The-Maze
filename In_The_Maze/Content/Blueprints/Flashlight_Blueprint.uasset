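; Flashlight pickup actor that spins a fixed step every tick and grants the flashlight when FirstPersonCharacter overlaps it.
; On overlap it sets the character's flashlight flags and shows its FlashlightOff component.
; It then saves flashlight ownership to the MainLevel slot for use between levels and destroys itself.
; The save uses a newly created ITM_SaveData object rather than loading the existing one.
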(event `self.ReceiveActorBeginOverlap`
  (params (OtherActor :type "Actor Object Reference"))
  ;[1 1 1] Anthony- Initial Light Stuff
  (bind _asfirst_person_character (cast `/Game/FirstPersonBP/Blueprints/FirstPersonCharacter` OtherActor))
  (set `/Game/FirstPersonBP/Blueprints/FirstPersonCharacter.hasFlashlight` true _asfirst_person_character)
  (set `/Game/FirstPersonBP/Blueprints/FirstPersonCharacter.flashlightOn/Off` true _asfirst_person_character)
  (`SceneComponent.SetVisibility` (`/Game/FirstPersonBP/Blueprints/FirstPersonCharacter.Flashlight_Off` _asfirst_person_character) true false)
  ;[1 1 1] Archie- Saving Between Levels
  (bind _returnvalue (`GameplayStatics.CreateSaveGameObject` "/Game/SavaData/ITM_SaveData.ITM_SaveData_C"))
  (set `/Game/SavaData/ITM_SaveData.hasFlashlightFromLevel` true _returnvalue)
  (`GameplayStatics.SaveGameToSlot` _returnvalue "MainLevel")
  (`self.K2_DestroyActor`))

(event `self.ReceiveTick`
  (params (DeltaSeconds :type "Float (single-precision)"))
  ;[1 1 1] Anthony- Initial Light Stuff
  (`self.K2_AddActorLocalRotation` (struct :`Yaw` 1.0)))

(fn `UserConstructionScript`)