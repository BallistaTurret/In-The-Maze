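; BatterySpawner is an actor Blueprint that spawns Battery_Blueprint actors at its root transform.
; Each Tick runs IsOverlappingActor with no actor specified, spawns a battery when it returns false, and sets HasBattery on both branches.
; The Delay after spawning leads to nothing, so it does not throttle spawns.
; HasBattery is never read in live logic, and several leftover node chains are disconnected.
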(event `self.ReceiveBeginPlay`)

(event `self.ReceiveTick`
  (params (DeltaSeconds :type "Float (single-precision)"))
  (if (`self.IsOverlappingActor` null)
    (set `self.hasBattery` true)
    (else
      (`|SpawnActorFromClass` "/Game/Blueprints/Battery_Blueprint.Battery_Blueprint_C" (`SceneComponent.K2_GetComponentToWorld` (`self.DefaultSceneRoot`)) "Undefined" "OverrideRootScale" null null)
      (set `self.hasBattery` true)
      (`KismetSystemLibrary.Delay` 2.0))))

(fn `UserConstructionScript`)