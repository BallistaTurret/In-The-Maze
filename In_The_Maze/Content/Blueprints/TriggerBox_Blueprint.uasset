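; TriggerBox_Blueprint is a level-transition trigger that saves player progress before loading another map.
; When a FirstPersonCharacter overlaps it, it copies Lives, Stamina and Battery into a newly created ITM_SaveData object.
; It writes that object to the MainLevel slot, then opens the level named by LevelToTransport.
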(event `self.ReceiveActorBeginOverlap`
  (params (OtherActor :type "Actor Object Reference"))
  ;[1 1 1] Archie: Set Level and Save L:ives, Stamina, and Battery life Between Levels
  (bind _returnvalue (`GameplayStatics.CreateSaveGameObject` "/Game/SavaData/ITM_SaveData.ITM_SaveData_C"))
  (bind _asfirst_person_character (cast `/Game/FirstPersonBP/Blueprints/FirstPersonCharacter` OtherActor))
  (set `/Game/SavaData/ITM_SaveData.SavedLives` (`/Game/FirstPersonBP/Blueprints/FirstPersonCharacter.lives` _asfirst_person_character) _returnvalue)
  (set `/Game/SavaData/ITM_SaveData.SavedStamina` (`/Game/FirstPersonBP/Blueprints/FirstPersonCharacter.Stamina` _asfirst_person_character) _returnvalue)
  (set `/Game/SavaData/ITM_SaveData.SavedBattery` (`/Game/FirstPersonBP/Blueprints/FirstPersonCharacter.battery` _asfirst_person_character) _returnvalue)
  (`GameplayStatics.SaveGameToSlot` _returnvalue "MainLevel")
  (`GameplayStatics.OpenLevel` (`self.LevelToTransport`)))

(fn `UserConstructionScript`)