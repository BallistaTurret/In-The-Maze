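; Message actor that shows a letter on screen while the player stands within it.
; When an actor tagged Player begins overlapping, it creates LetterWidget1, adds it to the viewport and plays a 2D sound.
; Any end overlap removes the widget, with no tag check.
; The Interact input only checks the Overlapping actor's tag and does nothing, as the nodes that set that variable are unwired.
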(event `InputAction|Interact`
  (params (Key :type "Key Structure"))
  (:`Pressed`
    (if (`self.ActorHasTag` (`self.Overlapping`) "Player")
      _)))

(event `self.ReceiveActorBeginOverlap`
  (params (OtherActor :type "Actor Object Reference"))
  (if (`self.ActorHasTag` OtherActor "Player")
    (bind _returnvalue (`|CreateWidget` "/Game/UI/LetterWidget1.LetterWidget1_C"))
    (`UserWidget.AddToViewport` _returnvalue 0)
    (`GameplayStatics.PlaySound2D` "/Game/Audio/Gorilla-SoundBible_com-1576451741.Gorilla-SoundBible_com-1576451741" 1.0 1.0 0.0 null null)))

(event `self.ReceiveActorEndOverlap`
  (params (OtherActor :type "Actor Object Reference"))
  (`Widget.RemoveFromParent` (stale `self.ReceiveActorBeginOverlap` _returnvalue)))

(fn `UserConstructionScript`)